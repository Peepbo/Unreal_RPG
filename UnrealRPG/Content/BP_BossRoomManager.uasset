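; Boss room manager actor that starts and ends a boss encounter.
; A box overlap sets the combat flag, then for a player character reveals the portal and light, activates the boss on them, shows its HUD health bar and fades in audio after a delay.
; While in combat, Tick watches the boss's target; once it is invalid, the audio fades out, portal, light and bar hide, and combat resets.
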(event OnComponentBeginOverlap(Box)
  (params (OverlappedComponent :type Primitive%20Component%20Object%20Reference) (OtherActor :type Actor%20Object%20Reference) (OtherComp :type Primitive%20Component%20Object%20Reference) (OtherBodyIndex :type Integer) (bFromSweep :type Boolean) (SweepResult :type Hit%20Result%20Structure%20%28by%20ref%29))
  (if (not (Variables|Default|GetbCombat))
    (Variables|Default|SetbCombat true)
    (bind _asplayer_character (Utilities|Casting|CastToPlayerCharacter OtherActor))
    (Variables|Default|SetPlayer _asplayer_character)
    (Utilities|FlowControl|Sequence
      (:then_0
        (bind _portal (Variables|Default|GetPortal)
          (:then
            (Rendering|SetActorHiddenInGame _portal false))
          (:else)))
      (:then_1
        (bind _light (Variables|Default|GetLight)
          (:then
            (Rendering|SetActorHiddenInGame _light false))
          (:else)))
      (:then_2
        (bind _audio (Variables|Default|GetAudio)
          (:then
            (Utilities|FlowControl|Delay 2.3)
            (Audio|Components|Audio|Play _audio 0.0)
            (Audio|Components|Audio|FadeIn _audio 1.5 0.7 0.0 "Linear" :!class /Script/Engine.AudioComponent))
          (:else)))
      (:then_3
        (bind _boss (Variables|Default|GetBoss)
          (:then
            (Class|Enemy|ActiveEnemy _boss (Variables|Default|GetPlayer)))
          (:else)))
      (:then_4
        (bind _hudoverlay (Variables|/Game/_Game/PlayerData/GI_BasicGameIntance.GI_BasicGameIntance_C|GetHudOverlay (.AsGI%20Basic%20Game%20Intance (Utilities|Casting|CastToGI_BasicGameIntance (Game|GetGameInstance))))
          (:then
            (Default|InitBossHealthBar _hudoverlay (Variables|Default|GetBoss))
            (Widget|SetVisibility (Variables|/Game/_Game/HUD/HUDOverlay.HUDOverlay_C|GetBP_BossHealthBar _hudoverlay) "Visible"))
          (:else))))))

(event EventBeginPlay
  (Utilities|FlowControl|Sequence
    (:then_0
      (bind _portal (Variables|Default|GetPortal)
        (:then
          (Rendering|SetActorHiddenInGame _portal true))
        (:else)))
    (:then_1
      (bind _light (Variables|Default|GetLight)
        (:then
          (Rendering|SetActorHiddenInGame _light true))
        (:else)))))

(event Collision|EventActorBeginOverlap
  (params (OtherActor :type Actor%20Object%20Reference)))

(event EventTick
  (params (DeltaSeconds :type Float%20%28single-precision%29))
  (if (Variables|Default|GetbCombat)
    (Variables|/Script/UnrealRPG.Enemy|GetTarget (Variables|Default|GetBoss)
      (:then)
      (:else
        (Audio|Components|Audio|FadeOut (Variables|Default|GetAudio) 2.0 0.0 "Linear" :!class /Script/Engine.AudioComponent)
        (Utilities|FlowControl|Sequence
          (:then_0
            (bind _portal (Variables|Default|GetPortal)
              (:then
                (Rendering|SetActorHiddenInGame _portal true))
              (:else)))
          (:then_1
            (bind _light (Variables|Default|GetLight)
              (:then
                (Rendering|SetActorHiddenInGame _light true))
              (:else)))
          (:then_2
            (Variables|Default|SetbCombat false)
            (Variables|Default|SetPlayer 0))
          (:then_3
            (bind _hudoverlay (Variables|/Game/_Game/PlayerData/GI_BasicGameIntance.GI_BasicGameIntance_C|GetHudOverlay (.AsGI%20Basic%20Game%20Intance (Utilities|Casting|CastToGI_BasicGameIntance (Game|GetGameInstance))))
              (:then
                (Widget|SetVisibility (Variables|/Game/_Game/HUD/HUDOverlay.HUDOverlay_C|GetBP_BossHealthBar _hudoverlay) "Hidden"))
              (:else))))))))

(fn ConstructionScript)