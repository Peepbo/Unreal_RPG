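; Level enemy manager that persists which enemies and bosses are still alive per level and save slot, registering itself with the game instance.
; Keeps separate enemy and boss arrays, each saved as a BP_EnemyIngameData survival array under its own slot name.
; If either save is missing, it gathers and indexes all Enemy actors and creates fresh saves.
; Otherwise it disables dead entries by array index, also force-killing regular enemies.
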(event Custom|DataRetarget
  (bind _outactors (Utilities|FindAllEnemyType))
  (for _array_element _outactors
    (Utilities|Casting|CastToBoss _array_element
      (:then
        (Utilities|Array|Add (Variables|Default|GetBossArr) _array_element))
      (:CastFailed
        (Utilities|Array|Add (Variables|Default|GetEnemyArr) _array_element))))
  (Utilities|SetEnemyIndex)
  (Utilities|NewEnemyIngameData))

(event EventBeginPlay
  (Utilities|UpdateLevelNameandSaveSlot)
  (bind _returnvalue (SaveGame|DoesSaveGameExist (Utilities|GetDataName false)))
  (bind _returnvalue_2 (SaveGame|DoesSaveGameExist (Utilities|GetDataName true)))
  (if (and _returnvalue_2 _returnvalue)
    (Utilities|LoadandApplyIngameData)
    (else
      (CallFunction|DataRetarget)))
  (Utilities|SendManagerData))

(event Collision|EventActorBeginOverlap
  (params (OtherActor :type Actor%20Object%20Reference)))

(event EventTick
  (params (DeltaSeconds :type Float%20%28single-precision%29)))

(fn ConstructionScript)

(fn SaveIngameData
  (Utilities|UpdateLevelNameandSaveSlot)
  (Utilities|FlowControl|Sequence
    (:then_0
      (bind _returnvalue (SaveGame|DoesSaveGameExist (Utilities|GetDataName false)))
      (if _returnvalue
        (bind _returnvalue_2 (SaveGame|LoadGamefromSlot (Utilities|GetDataName false)))
        (bind _asbp_enemy_ingame_data (Utilities|Casting|CastToBP_EnemyIngameData _returnvalue_2))
        (Default|UpdateData _asbp_enemy_ingame_data (Variables|Default|GetEnemyArr))
        (SaveGame|SaveGametoSlot _asbp_enemy_ingame_data (Utilities|GetDataName false))))
    (:then_1
      (bind _returnvalue_3 (SaveGame|DoesSaveGameExist (Utilities|GetDataName true)))
      (if _returnvalue_3
        (bind _returnvalue_4 (SaveGame|LoadGamefromSlot (Utilities|GetDataName true)))
        (bind _asbp_enemy_ingame_data_2 (Utilities|Casting|CastToBP_EnemyIngameData _returnvalue_4))
        (Default|UpdateData _asbp_enemy_ingame_data_2 (Variables|Default|GetBossArr))
        (SaveGame|SaveGametoSlot _asbp_enemy_ingame_data_2 (Utilities|GetDataName true))))))

(fn ResetData
  (Utilities|UpdateLevelNameandSaveSlot)
  (Utilities|NewEnemyIngameData))

(fn LoadData
  (Utilities|UpdateLevelNameandSaveSlot)
  (bind _returnvalue (SaveGame|DoesSaveGameExist (Utilities|GetDataName false)))
  (bind _returnvalue_2 (SaveGame|DoesSaveGameExist (Utilities|GetDataName true)))
  (if (and _returnvalue_2 _returnvalue)
    (Utilities|LoadandApplyIngameData)
    (else
      (CallFunction|DataRetarget)))
  (Utilities|SendManagerData))