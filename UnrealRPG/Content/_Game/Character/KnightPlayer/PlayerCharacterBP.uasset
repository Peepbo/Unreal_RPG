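; Player character Blueprint for the knight, mainly linking the character to its HUD.
; BeginPlay caches the HUDOverlay from the MeleePlayerController, and two events forward left and right item icon updates to it.
; Disconnected lock-on logic remains: a sphere overlap picks the nearest Enemy within a view cone, then control rotation lerps toward its widget with clamped pitch.
; That targeting code never runs, and Tick is empty.
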(event EventBeginPlay
  (bind _asmelee_player_controller (Utilities|Casting|CastToMeleePlayerController (Game|GetPlayerController 0)))
  (bind _ashudoverlay (Utilities|Casting|CastToHUDOverlay (Variables|/Script/UnrealRPG.MeleePlayerController|GetHUDOverlay _asmelee_player_controller)))
  (Variables|Default|SetOverlay _ashudoverlay))

(event Collision|EventActorBeginOverlap
  (params (OtherActor :type Actor%20Object%20Reference)))

(event EventTick
  (params (DeltaSeconds :type Float%20%28single-precision%29)))

(event EventUpdateLeftItemIcon
  (bind _overlay (Variables|Default|GetOverlay))
  (Utilities|IsValid _overlay
    (:Is%20Valid
      (Default|UpdateLeftItemIcon _overlay))))

(event EventUpdateRightItemIcon
  (bind _overlay (Variables|Default|GetOverlay))
  (Utilities|IsValid _overlay
    (:Is%20Valid
      (Default|UpdateRightItemIcon _overlay))))

(event Input|KeyboardEvents|K
  (params (Key :type Key%20Structure :default "None")))

(fn ConstructionScript)