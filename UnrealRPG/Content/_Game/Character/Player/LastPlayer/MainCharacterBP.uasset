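; Player character Blueprint that loads its data from the game instance and links the character to the HUD.
; BeginPlay initializes PlayerData from GI_BasicGameIntance, then caches the HUD overlay from the melee player controller.
; Left, right and bottom item icon events forward to that overlay when valid.
; The K key prints the player name and opens the player data widget in save mode with the cursor shown and UI-only input.
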(event EventBeginPlay
  (bind _returnvalue (Game|GetGameInstance))
  (bind (_asgi_basic_game_intance _bsuccess) (Utilities|Casting|CastToGI_BasicGameIntance _returnvalue))
  (if _bsuccess
    (Class|PlayerCharacter|InitPlayerData (Variables|/Game/_Game/PlayerData/GI_BasicGameIntance.GI_BasicGameIntance_C|GetPlayerData _asgi_basic_game_intance))
    (bind _asmelee_player_controller (Utilities|Casting|CastToMeleePlayerController (Pawn|GetController)))
    (bind _ashudoverlay (Utilities|Casting|CastToHUDOverlay (Variables|/Script/UnrealRPG.MeleePlayerController|GetHUDOverlay _asmelee_player_controller)))
    (Variables|Default|SetOverlay _ashudoverlay)))

(event Collision|EventActorBeginOverlap
  (params (OtherActor :type Actor%20Object%20Reference)))

(event EventTick
  (params (DeltaSeconds :type Float%20%28single-precision%29)))

(event EventUpdateLeftItemIcon
  (bind _overlay (Variables|Default|GetOverlay))
  (Utilities|IsValid _overlay
    (:Is%20Valid
      (Default|UpdateLeftItemIcon _overlay))))

(event EventUpdateRightItemIcon
  (bind _overlay (Variables|Default|GetOverlay))
  (Utilities|IsValid _overlay
    (:Is%20Valid
      (Default|UpdateRightItemIcon _overlay))))

(event EventUpdateBottomItemIcon
  (bind _overlay (Variables|Default|GetOverlay))
  (Utilities|IsValid _overlay
    (:Is%20Valid
      (Default|UpdateBottomItemIcon _overlay))))

(event Input|KeyboardEvents|K
  (params (Key :type Key%20Structure :default "None"))
  (:Pressed
    (Development|PrintString (Utilities|String|Append "Player Name : " (Utilities|String|ToString(Name) (.name (Variables|Default|GetPlayerData)))))
    (Variables|/Script/Engine.PlayerController|SetbShowMouseCursor (Game|GetPlayerController 0) true)
    (bind _returnvalue (UserInterface|CreateWidget "/Game/_Game/HUD/MainMenu/PlayerDataViewWidget.PlayerDataViewWidget_C"))
    ;[1 1 1] SaveMode
    (Default|InitWidgetSetting _returnvalue true)
    (Input|SetInputModeUIOnly (Game|GetPlayerController 0) 0 "LockAlways")
    (UserInterface|Viewport|AddtoViewport _returnvalue 0)))

(fn ConstructionScript)