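; Boss projectile that accelerates toward a maximum speed along its local X axis and damages the player on contact.
; Tick moves it and sphere-traces at its location; it passes through a rolling player, while any other hit triggers explosion effects, hides the sphere and stops movement.
; A delay loop then fades the Niagara "Fire" parameter before destroying the actor.
; The construction script applies Size and initial fire intensity.
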(event Custom|NiagaraLerpEvent
  (Variables|Default|SetNiagaraParam 0.5)
  (bind _output_get (Variables|Default|SetNiagaraParam (Math|Float|Lerp (Variables|Default|GetNiagaraParam) 0.0 0.05) :!label _label))
  (if (Math|Float|NearlyEqual(Float) (Variables|Default|GetNiagaraParam) 0.0 0.001)
    (Actor|DestroyActor)
    (else
      (Effects|Components|ParticleSystem|SetFloatParameter (Variables|Default|GetNiagara) "Fire" _output_get)
      (Utilities|FlowControl|Delay (Utilities|Time|GetWorldDeltaSeconds))
      (goto _label))))

(event EventBeginPlay)

(event EventTick
  (params (DeltaSeconds :type Float%20%28single-precision%29))
  (bind _returnvalue (Transformation|GetActorLocation))
  (if (not (Variables|Default|GetbStop))
    (bind _output_get (Variables|Default|SetSpeed (Math|Float|Lerp (Variables|Default|GetSpeed) (Variables|Default|GetMaximumSpeed) (* DeltaSeconds 2.0))))
    (Transformation|AddActorLocalOffset (Math|Vector|MakeVector _output_get 0.0 0.0) false false)
    (bind (_outhit _returnvalue_2) (Collision|SphereTraceByChannel _returnvalue _returnvalue 1e+02 "TraceTypeQuery1" false 0 "None"))
    (if _returnvalue_2
      (bind _asplayer_character (Utilities|Casting|CastToPlayerCharacter (.HitActor (Collision|BreakHitResult _outhit)))
        (:then
          (if (Utilities|Enum|NotEqual(Enum) (Variables|/Script/UnrealRPG.MeleeCharacter|GetCombatState _asplayer_character) "ECS_Roll")
            (Game|Damage|ApplyDamage _asplayer_character (Variables|Default|GetDamage) 0 (Components|GetOwner) "/Script/Engine.DamageType")
            (Development|PrintString (Utilities|GetDisplayName (.HitActor (Collision|BreakHitResult _outhit))) true true "(R=1.000000,G=0.114580,B=0.000000,A=1.000000)" :!label _label)
            (Effects|SpawnEmitteratLocation "/Game/FXAsset/FXVarietyPack/Particles/P_ky_explosion.P_ky_explosion" (.ImpactPoint (Collision|BreakHitResult _outhit)))
            (Niagara|SpawnSystematLocation "/Game/_Game/FX/Boss/Projectile/NS_ProjectileBoom.NS_ProjectileBoom" (Transformation|GetWorldLocation (Variables|Default|GetSphere)) "0.000000,-90.000000, 0")
            (Rendering|SetVisibility (Variables|Default|GetSphere) false false)
            (Variables|Default|SetbStop true)
            (CallFunction|NiagaraLerpEvent)))
        (:CastFailed
          (goto _label))))))

(fn ConstructionScript
  (Effects|Components|ParticleSystem|SetFloatParameter (Variables|Default|GetNiagara) "Fire" (Variables|Default|GetNiagaraParam))
  (Effects|Components|ParticleSystem|SetFloatParameter (Variables|Default|GetNiagara) "Size" (Variables|Default|GetSize))
  (Transformation|SetRelativeScale3D (Variables|Default|GetSphere) (* "1.000000,1.000000,1.000000" (Math|Conversions|ToVector(Float) (Variables|Default|GetSize)))))