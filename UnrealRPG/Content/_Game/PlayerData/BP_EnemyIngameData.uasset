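; BP_EnemyIngameData records which enemies are still alive as an array of survival flags, indexed by enemy.
; Init Data resizes the array to a given count and marks every entry as surviving.
; UpdateData walks a supplied enemy array and clears the flag at the index of each dying enemy; it never sets a flag back to true.
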(fn InitData
  (params (Size :type Integer))
  (Utilities|Array|Resize (Variables|Default|GetSurvivalArr) Size)
  (for (_ _array_index) (Variables|Default|GetSurvivalArr)
    (|SetBy-RefVar (Utilities|Array|Get(acopy) (Variables|Default|GetSurvivalArr) _array_index) true)))

(fn UpdateData
  (params (Enemies :type Array%20of%20Enemy%20Object%20References))
  (for (_array_element _array_index) Enemies
    (if (Variables|/Script/UnrealRPG.MeleeCharacter|GetbDying _array_element)
      (Utilities|Array|SetArrayElem (Variables|Default|GetSurvivalArr) _array_index false))))