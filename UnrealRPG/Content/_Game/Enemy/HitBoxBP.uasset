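; HitBoxBP is an enemy hit box actor that damages the player character on overlap, then goes on a timed cooldown.
; An overlap applies damage with an attack type, passes the box's location to the player as a hit point, and disables collision and the mesh.
; Tick then counts up, showing whole seconds on a text render, and re-arms the box with a ready message and color change once PrepareTime elapses.
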(event EventBeginPlay)

(event Collision|EventActorBeginOverlap
  (params (OtherActor :type Actor%20Object%20Reference))
  (bind _asplayer_character (Utilities|Casting|CastToPlayerCharacter OtherActor))
  (Class|MeleeCharacter|CustomApplyDamage _asplayer_character _asplayer_character (Variables|Default|GetDamage) self (Variables|Default|GetAttackType))
  (Class|PlayerCharacter|SetHitPointTest _asplayer_character (Transformation|GetActorLocation))
  (Variables|Default|SetbPrepare false)
  (Collision|SetActorEnableCollision false)
  (Rendering|SetVisibility (Variables|Default|GetHitMesh) false false)
  (Rendering|Components|TextRender|SetTextRenderColor (Variables|Default|GetTextRender) (Variables|Default|GetColor%201)))

(event EventTick
  (params (DeltaSeconds :type Float%20%28single-precision%29))
  (if (not (Variables|Default|GetbPrepare))
    (Variables|Default|SetNowTime (+ (Variables|Default|GetNowTime) DeltaSeconds))
    (if (>= (Variables|Default|GetNowTime) (Variables|Default|GetPrepareTime))
      (Variables|Default|SetbPrepare true)
      (Collision|SetActorEnableCollision true)
      (Rendering|SetVisibility (Variables|Default|GetHitMesh) true false)
      (Variables|Default|SetNowTime 0.0)
      (Rendering|Components|TextRender|SetText (Variables|Default|GetTextRender) (Variables|Default|GetReady%20Text))
      (Rendering|Components|TextRender|SetTextRenderColor (Variables|Default|GetTextRender) (Variables|Default|GetColor%202))
      (else
        (Rendering|Components|TextRender|SetText (Variables|Default|GetTextRender) (Utilities|Text|ToText(String) (Class|KismetMathLibrary|FTrunc64 (Variables|Default|GetNowTime))))))))

(fn ConstructionScript)