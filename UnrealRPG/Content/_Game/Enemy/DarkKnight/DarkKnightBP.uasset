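; Dark Knight enemy Blueprint that handles its health bar and weapon visibility.
; On BeginPlay it sets itself as the Enemy on its health bar widget, then passes the Weapon component to GetWeaponMesh.
; Events hide the health bar widget and show or hide the Weapon and the back-carried WeaponCase independently, with no combat or AI logic in these graphs.
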(event EventBeginPlay
  (bind _asenemy_health_bar_bp (Utilities|Casting|CastToEnemyHealthBarBP (UserInterface|GetUserWidgetObject (Variables|Default|GetHealth%20Bar))))
  (Variables|/Game/_Game/HUD/EnemyHealthBarBP.EnemyHealthBarBP_C|SetEnemy _asenemy_health_bar_bp self)
  (Class|DarkKnight|GetWeaponMesh (Variables|Default|GetWeapon)))

(event Collision|EventActorBeginOverlap
  (params (OtherActor :type Actor%20Object%20Reference)))

(event EventTick
  (params (DeltaSeconds :type Float%20%28single-precision%29)))

(event EventHideHealthBar
  (bind _health_bar (Variables|Default|GetHealth%20Bar))
  (Utilities|IsValid _health_bar
    (:Is%20Valid
      (Widget|SetVisibility (UserInterface|GetUserWidgetObject _health_bar) "Hidden"))))

(event EventHideBackWeapon
  (Rendering|SetVisibility (Variables|Default|GetWeaponCase) false false))

(event EventHideWeapon
  (Rendering|SetVisibility (Variables|Default|GetWeapon) false false))

(event EventShowWeapon
  (Rendering|SetVisibility (Variables|Default|GetWeapon) true false))

(event EventShowBackWeapon
  (Rendering|SetVisibility (Variables|Default|GetWeaponCase) true false))

(fn ConstructionScript)