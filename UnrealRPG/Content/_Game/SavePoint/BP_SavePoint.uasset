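; Save point actor that offers its ResponPoint location to a PlayerCharacter standing inside its Sphere trigger.
; On overlap it enables the player's event flag and passes that location as the close save point; leaving disables the flag and resets the location to zero.
; While the player is near, the PlayerCloseEffect timeline bobs the mesh vertically, replaying on finish until the player leaves.
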(event OnComponentBeginOverlap(Sphere)
  (params (OverlappedComponent :type Primitive%20Component%20Object%20Reference) (OtherActor :type Actor%20Object%20Reference) (OtherComp :type Primitive%20Component%20Object%20Reference) (OtherBodyIndex :type Integer) (bFromSweep :type Boolean) (SweepResult :type Hit%20Result%20Structure%20%28by%20ref%29))
  (bind _asplayer_character (Utilities|Casting|CastToPlayerCharacter OtherActor))
  (Class|PlayerCharacter|SetEventAble _asplayer_character true)
  (Class|PlayerCharacter|SetCloseSavePoint _asplayer_character (Transformation|GetWorldLocation (Variables|Default|GetResponPoint)))
  (Variables|Default|SetbClosePlayer true)
  (bind _floating_mesh (Timeline|PlayerCloseEffect Play)
    (:Update
      (Transformation|SetRelativeLocation (Variables|Default|GetStaticMesh) (Math|Vector|MakeVector 0.0 0.0 (+ _floating_mesh 5e+01)) false false))
    (:Finished
      (if (Variables|Default|GetbClosePlayer)
        (CallFunction|Repeat)))))

(event OnComponentEndOverlap(Sphere)
  (params (OverlappedComponent :type Primitive%20Component%20Object%20Reference) (OtherActor :type Actor%20Object%20Reference) (OtherComp :type Primitive%20Component%20Object%20Reference) (OtherBodyIndex :type Integer))
  (bind _asplayer_character (Utilities|Casting|CastToPlayerCharacter OtherActor))
  (Class|PlayerCharacter|SetEventAble _asplayer_character false)
  (Class|PlayerCharacter|SetCloseSavePoint _asplayer_character "0, 0, 0")
  (Variables|Default|SetbClosePlayer false))

(event Custom|Repeat
  (bind _floating_mesh (Timeline|PlayerCloseEffect PlayFromStart)
    (:Update
      (Transformation|SetRelativeLocation (Variables|Default|GetStaticMesh) (Math|Vector|MakeVector 0.0 0.0 (+ _floating_mesh 5e+01)) false false))
    (:Finished
      (if (Variables|Default|GetbClosePlayer)
        (CallFunction|Repeat)))))

(event EventBeginPlay)

(event Collision|EventActorBeginOverlap
  (params (OtherActor :type Actor%20Object%20Reference)))

(event EventTick
  (params (DeltaSeconds :type Float%20%28single-precision%29)))

(fn ConstructionScript)