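; Enemy AI controller that tracks the player's MeleeCharacter through AI Perception and writes the result to the Blackboard.
; Sensing the character sets HasLineOfSight and EnemyActor and cancels any pending lose-target timer.
; Losing it starts a four-second timer that clears both keys, so the enemy keeps its target briefly after losing perception.
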(event OnTargetPerceptionUpdated(AIPerception)
  (params (Actor :type Actor%20Object%20Reference) (Stimulus :type AI%20Stimulus%20Structure))
  (bind _blackboardcomponent (Variables|Default|GetBlackboardComponent))
  (Utilities|Casting|CastToMeleeCharacter Actor)
  (if (.bSuccessfullySensed (Utilities|Struct|BreakAIStimulus Stimulus))
    (Utilities|Time|ClearandInvalidateTimerbyHandle (Variables|Default|GetEnemyTimer))
    (AI|Components|Blackboard|SetValueasBool _blackboardcomponent (Variables|Default|GetHas%20Line%20Of%20Sight) true)
    (AI|Components|Blackboard|SetValueasObject _blackboardcomponent (Variables|Default|GetEnemy%20Actor) Actor)
    (else
      (bind _returnvalue (Utilities|Time|SetTimerbyEvent (delegate Custom|StartEnemyTimer) 4.0))
      (Variables|Default|SetEnemyTimer _returnvalue))))

(event Custom|StartEnemyTimer
  (bind _blackboardcomponent (Variables|Default|GetBlackboardComponent))
  (AI|Components|Blackboard|SetValueasBool _blackboardcomponent (Variables|Default|GetHas%20Line%20Of%20Sight) false)
  (AI|Components|Blackboard|SetValueasObject _blackboardcomponent (Variables|Default|GetEnemy%20Actor) 0))

(event EventBeginPlay)

(event EventTick
  (params (DeltaSeconds :type Float%20%28single-precision%29)))

(fn ConstructionScript)